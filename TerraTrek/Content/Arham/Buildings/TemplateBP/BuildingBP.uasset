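; Building template that reacts to an Interact event and spawns a BuildingItselfBP at its root location after one second.
; A Box overlap tracks the OtherActor used by the interaction.
; With enough game-mode EnergyPoints and a ThirdPersonCharacter overlapping, the building offsets itself along local X.
; An overlapping Sedan is teleported aside along Y; this and the delayed spawn ignore the energy check.
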(event `/Game/Arham/Player/Interact.Interact`
  (bind _other_actor (`self.Other Actor`))
  (`|ExecutionSequence`
    (:`then_0`
      (bind _returnvalue (`GameplayStatics.GetActorOfClass` "/Game/Arham/Player/ThirdPersonGameMode.ThirdPersonGameMode_C"))
      (set `self.Check` (> (`/Game/Arham/Player/ThirdPersonGameMode.EnergyPoints` _returnvalue) 9)))
    (:`then_1`
      (if (`self.Check`)
        (cast `/Game/Arham/Player/ThirdPersonCharacter` (`self.Other Actor`))
        (`self.K2_AddActorLocalOffset` (400.0 0.0 0.0) false true)))
    (:`then_2`
      (bind _assedan (cast `/Game/Arham/VehicleBP/Sedan/Sedan` _other_actor))
      (bind (_returnvalue_x _returnvalue_y) (`KismetMathLibrary.BreakVector` (`self.K2_GetActorLocation` _assedan)))
      (`self.K2_SetActorLocation` _other_actor (`KismetMathLibrary.MakeVector` _returnvalue_x (+ _returnvalue_y 700.0) 100.0) false true))
    (:`then_3`
      (`KismetSystemLibrary.Delay` 1.0)
      (`|SpawnActorFromClass` "/Game/Arham/Buildings/TemplateBP/BuildingItselfBP.BuildingItselfBP_C" (`KismetMathLibrary.Conv_VectorToTransform` (`SceneComponent.K2_GetComponentLocation` (`self.DefaultSceneRoot`))) "Undefined" "OverrideRootScale" null null))))

(event `self.Box.OnComponentBeginOverlap`
  (params (OverlappedComponent :type "PrimitiveComponent Object Reference") (OtherActor :type "Actor Object Reference") (OtherComp :type "PrimitiveComponent Object Reference") (OtherBodyIndex :type Integer) (bFromSweep :type Boolean) (SweepResult :type "HitResult Structure (by ref)"))
  ;[1 1 1] Collision
  (set `self.Other Actor` OtherActor))

(event `self.Box.OnComponentEndOverlap`
  (params (OverlappedComponent :type "PrimitiveComponent Object Reference") (OtherActor :type "Actor Object Reference") (OtherComp :type "PrimitiveComponent Object Reference") (OtherBodyIndex :type Integer))
  ;[1 1 1] Collision
  (set `self.Other Actor` (`self.Empty`)))

(fn `UserConstructionScript`)